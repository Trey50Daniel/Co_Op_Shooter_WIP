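; Enemy actor for a first-person game that takes damage and scores points for the player.
; Its TakeDamage event subtracts from CurrentHealth and calls AddPoints on the player character for every hit, including the lethal one.
; When health reaches zero or below, it destroys itself, decrements EnemiesLeft on BP_FirstPersonGameMode and calls CheckEnemiesLeft there.
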(event Custom|TakeDamage
  (params (Damage :type Float%20%28double-precision%29))
  (Variables|Default|SetCurrent_Health (- (Variables|Default|GetCurrent_Health) Damage))
  (if (> (Variables|Default|GetCurrent_Health) 0.0)
    (CallFunction|AddPlayerPoints)
    (else
      (CallFunction|AddPlayerPoints)
      (Actor|DestroyActor)
      (bind _asbp_first_person_game_mode (Utilities|Casting|CastToBP_FirstPersonGameMode (Game|GetGameMode)))
      (Variables|/Game/FirstPerson/Blueprints/BP_FirstPersonGameMode.BP_FirstPersonGameMode_C|SetEnemiesLeft _asbp_first_person_game_mode (- (Variables|/Game/FirstPerson/Blueprints/BP_FirstPersonGameMode.BP_FirstPersonGameMode_C|GetEnemiesLeft _asbp_first_person_game_mode) 1.0))
      (Default|CheckEnemiesLeft _asbp_first_person_game_mode))))

(event EventBeginPlay)

(event Collision|EventActorBeginOverlap
  (params (OtherActor :type Actor%20Object%20Reference)))

(event EventTick
  (params (DeltaSeconds :type Float%20%28single-precision%29)))

(fn ConstructionScript)

(fn AddPlayerPoints
  (bind _asbp_first_person_character (Utilities|Casting|CastToBP_FirstPersonCharacter (Game|GetPlayerCharacter 0)))
  (Default|AddPoints _asbp_first_person_character))